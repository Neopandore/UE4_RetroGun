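; BP_RetroPawn is a player pawn that moves around the screen and fires an attached weapon.
; BeginPlay spawns BP_MotherWeapon on WeaponAttach; primary input or an auto-fire toggle starts and stops it.
; Axis input snaps to full or zero speed, scales by delta time and moves only within projected screen bounds.
; Secondary fire, triggered by input or by touch when armed, is a placeholder print that clears the armed flag.
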(event `self.ReceiveBeginPlay`
  (bind _returnvalue (`|SpawnActorFromClass` "/Game/10_Blueprints/13_Weapons/BP_MotherWeapon.BP_MotherWeapon_C" (`KismetMathLibrary.MakeTransform` (0.0 0.0 0.0)) "AlwaysSpawn" "OverrideRootScale" self null))
  (bind _output_get (set `self.Weapon` _returnvalue))
  (`self.K2_AttachToComponent` _output_get (`self.WeaponAttach`) "None" "SnapToTarget" "SnapToTarget" "SnapToTarget" false))

(event `InputAxis|Up`
  (params (AxisValue :type "Float (single-precision)"))
  (bind _scaledspeed (`self.SpeedScale` AxisValue true))
  (bind _inbounds (`self.CheckScreenBounds` _scaledspeed))
  (if _inbounds
    (`self.K2_AddActorWorldOffset` (`KismetMathLibrary.MakeVector` _scaledspeed) true)))

(event `InputAxis|Right`
  (params (AxisValue :type "Float (single-precision)"))
  (bind _scaledspeed (`self.SpeedScale` AxisValue))
  (bind _inbounds (`self.CheckScreenBounds` _scaledspeed "NewEnumerator1"))
  (if _inbounds
    (`self.K2_AddActorWorldOffset` (`KismetMathLibrary.MakeVector` 0.0 _scaledspeed) true)))

(event `InputAction|PrimaryFire`
  (params (Key :type "Key Structure"))
  (bind _weapon (`self.Weapon`))
  (:`Pressed`
    (`/Game/10_Blueprints/13_Weapons/BP_MotherWeapon.Start Firing` _weapon :!label _label))
  (:`Released`
    (`/Game/10_Blueprints/13_Weapons/BP_MotherWeapon.Stop Firing` _weapon :!label _label_2)))

(event `Switch Auto Fire`
  (bind _output_get (set `self.AutoFire` (not (`self.AutoFire`))))
  (if _output_get
    (goto _label)
    (else
      (goto _label_2))))

(event `Activate Secondary Fire`
  (set `self.SecondaryActive` true))

(event `InputAction|SecondaryFire`
  (params (Key :type "Key Structure"))
  (:`Pressed`
    (`self.Fire Secondary` :!label _label_3)))

(event `InputTouch`
  (params (Location :type "Vector Structure") (FingerIndex :type "ETouchIndex Enum"))
  (:`Pressed`
    (if (`self.SecondaryActive`)
      (goto _label_3))))

(event `Fire Secondary`
  (`KismetSystemLibrary.PrintString` "Hello" true false (struct :`G` 0.66 :`B` 1.0 :`A` 1.0) 5.0)
  (set `self.SecondaryActive` false))

(fn `CheckScreenBounds`
  (params (AxisValue :type "Float (double-precision)") (Direction :type "/Game/20_Data/00_MovementAxis_Enum Enum" :default "NewEnumerator0"))
  (returns (InBounds :type Boolean))
  (bind (_returnvalue_x _returnvalue_y) (`KismetMathLibrary.BreakVector2D` (`WidgetLayoutLibrary.GetViewportSize`)))
  (bind _verticalspeed (`self.VerticalSpeed`))
  (if (!= AxisValue 0.0)
    (bind _asplayer_controller (cast `PlayerController` (`self.GetController`)))
    (switch `/Game/20_Data/00_MovementAxis_Enum` Direction
      (:`NewEnumerator0`
        (if (> AxisValue 0.0)
          (bind _screenposition (`GameplayStatics.ProjectWorldToScreen` _asplayer_controller (`self.K2_GetActorLocation`)))
          (return (>= (- (`.Y` (`KismetMathLibrary.BreakVector2D` _screenposition)) _verticalspeed) 0.0))
          (else
            (return (<= (+ (`.Y` (`KismetMathLibrary.BreakVector2D` _screenposition)) _verticalspeed) _returnvalue_y)))))
      (:`NewEnumerator1`
        (if (> AxisValue 0.0)
          (return (<= (+ (`KismetMathLibrary.BreakVector2D` _screenposition) _verticalspeed) _returnvalue_x))
          (else
            (return (>= (- (`KismetMathLibrary.BreakVector2D` _screenposition) _verticalspeed) 0.0))))))))

(fn `SpeedScale`
  (params (AxisValue :type "Float (double-precision)") (Vertical :type Boolean))
  (returns (ScaledSpeed :type "Float (double-precision)"))
  (locals (RoundedAxisValue_Local :type "Float (double-precision)"))
  (bind _returnvalue (`GameplayStatics.GetWorldDeltaSeconds`))
  (bind _roundedaxisvalue_local (`local.RoundedAxisValue_Local`))
  (if (> AxisValue 0.05)
    (set `local.RoundedAxisValue_Local` 1.0)
    (elif (< AxisValue -0.05)
      (set `local.RoundedAxisValue_Local` -1.0)
      (else
        (set `local.RoundedAxisValue_Local` 0.0))))
  (if Vertical
    (return (* _roundedaxisvalue_local (`self.VerticalSpeed`) 100.0 _returnvalue))
    (else
      (return (* _roundedaxisvalue_local (`self.HorizontalSpeed`) 100.0 _returnvalue)))))

(fn `UserConstructionScript`)
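; Enemy actor that turns to face the player, travels to an assigned target point and takes damage.
; StartMoving sets the destination and resets health for new pawns.
; Tick yaws toward player 0 and moves independently of facing, with distance-scaled, capped speed that eases into the target.
; It starts disabled, and lethal damage fires OnDeath and disables it rather than destroying it, allowing reuse.
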(event `StartMoving`
  (params (TargetPoint :type "Actor Object Reference") (IsNewPawn :type Boolean))
  (set `self.TargetPoint` TargetPoint)
  (set `self.CanMove` true)
  (if IsNewPawn
    (set `self.CurrentHealth` (`self.BaseHealth`))))

(event `self.ReceiveTick`
  (params (DeltaSeconds :type "Float (single-precision)"))
  (`|ExecutionSequence`
    (:`then_0`
      (`self.RotateTo`))
    (:`then_1`
      (`self.MoveTo`))))

(event `/Game/20_Data/i_Damageable.i_TakesDamages`
  (params (DamageValue :type Integer))
  (bind _returnvalue (- (`self.CurrentHealth`) DamageValue))
  (if (<= _returnvalue 0)
    (`self.OnDeath`)
    (`/Game/20_Data/Lib_RetroGun.EnableActor` self)
    (else
      (set `self.CurrentHealth` _returnvalue))))

(fn `MoveTo`
  (bind _returnvalue (`self.K2_GetActorLocation`))
  (bind _maxspeed (`self.MaxSpeed`))
  (bind _returnvalue_2 (`self.K2_GetActorLocation` (`self.TargetPoint`)))
  (bind _returnvalue_3 (`KismetMathLibrary.Vector_Distance` _returnvalue _returnvalue_2))
  (bind _returnvalue_4 (`KismetMathLibrary.GetForwardVector` (`KismetMathLibrary.FindLookAtRotation` _returnvalue _returnvalue_2)))
  (bind _returnvalue_5 (* (`self.BaseSpeed`) (* _returnvalue_3 0.0025) 100.0 (`GameplayStatics.GetWorldDeltaSeconds`)))
  (if (`self.CanMove`)
    (if (not (`KismetMathLibrary.NearlyEqual_FloatFloat` _returnvalue_3 0.0 5.0))
      (if (> _returnvalue_5 _maxspeed)
        (`self.K2_AddActorWorldOffset` (* _returnvalue_4 _maxspeed))
        (else
          (`self.K2_AddActorWorldOffset` (* _returnvalue_4 _returnvalue_5))))
      (else
        (set `self.CanMove` false)))))

(fn `RotateTo`
  (bind _returnvalue (`self.K2_GetActorRotation`))
  (bind _returnvalue_2 (* (`self.RotationRate`) (`GameplayStatics.GetWorldDeltaSeconds`)))
  (bind _returnvalue_3 (`KismetMathLibrary.FindLookAtRotation` (`self.K2_GetActorLocation`) (`self.K2_GetActorLocation` (`GameplayStatics.GetPlayerPawn` 0))))
  (bind (_returnvalue_roll _returnvalue_pitch _returnvalue_yaw) (`KismetMathLibrary.BreakRotator` (`KismetMathLibrary.NormalizedDeltaRotator` _returnvalue_3 _returnvalue)))
  (if (!= _returnvalue_3 _returnvalue :`ErrorTolerance` 1.0)
    (if (> _returnvalue_yaw 0.0)
      (`self.K2_SetActorRotation` (`KismetMathLibrary.ComposeRotators` _returnvalue (`KismetMathLibrary.MakeRotator` 0.0 0.0 _returnvalue_2)))
      (else
        (`self.K2_SetActorRotation` (`KismetMathLibrary.NormalizedDeltaRotator` _returnvalue (`KismetMathLibrary.MakeRotator` 0.0 0.0 _returnvalue_2)))))))

(fn `UserConstructionScript`
  (`/Game/20_Data/Lib_RetroGun.EnableActor` self))
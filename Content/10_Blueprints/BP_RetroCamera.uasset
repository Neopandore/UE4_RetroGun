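; BP_RetroCamera manages player views, switching each controller between a top camera and a side camera.
; On BeginPlay it loops over the game mode's player count, binding CameraSwitch to each BP_RetroController's switch dispatcher and starting on the top view.
; It also attaches each pawn to itself and moves it to a fixed location.
; CameraSwitch blends the calling controller's view target over CameraBlendDelay, while ChangeCamera is an empty stub.
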(event `self.ReceiveBeginPlay`
  (bind _returnvalue (`GameModeBase.GetNumPlayers` (`GameplayStatics.GetGameMode`)))
  (for _index (range _returnvalue)
    (`|ExecutionSequence`
      (:`then_0`
        (bind _returnvalue_2 (`GameplayStatics.GetPlayerController` _index))
        (bind _asbp_retro_controller (cast `/Game/10_Blueprints/11_PlayerPawn/BP_RetroController` _returnvalue_2))
        (add `/Game/10_Blueprints/11_PlayerPawn/BP_RetroController.CameraSwitch_Dispatch` _asbp_retro_controller (delegate `CameraSwitch`)))
      (:`then_1`
        (`PlayerController.SetViewTargetWithBlend` _returnvalue_2 (`self.CameraTop`) 0.0 "VTBlend_Linear" 0.0 false)
        (bind _returnvalue_3 (`GameplayStatics.GetPlayerPawn` _index))
        (`self.K2_AttachToActor` _returnvalue_3 self "None" "KeepRelative" "KeepWorld" "KeepRelative" false)
        (`self.K2_SetActorLocation` _returnvalue_3 (0.0 -1000.0 1500.0) false false)))))

(event `CameraSwitch`
  (params (Controller :type "/Game/10_Blueprints/11_PlayerPawn/BP_RetroController Object Reference") (TopCamera :type Boolean))
  (bind _camerablenddelay (`self.CameraBlendDelay`))
  (if TopCamera
    (`PlayerController.SetViewTargetWithBlend` Controller (`self.CameraTop`) _camerablenddelay "VTBlend_Linear" 0.0 false)
    (else
      (`PlayerController.SetViewTargetWithBlend` Controller (`self.CameraSide`) _camerablenddelay "VTBlend_Linear" 0.0 false))))

(event `Change Camera`)

(fn `UserConstructionScript`)
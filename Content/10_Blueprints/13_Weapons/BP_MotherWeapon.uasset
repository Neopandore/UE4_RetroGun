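; Base weapon that fires pooled projectiles or box-trace lasers on a looping timer set by fire rate.
; Non-laser weapons pre-spawn a magazine of projectiles at BeginPlay, then cycle through it by teleporting and enabling them.
; FireWeapon supports single, alternate and simultaneous barrel modes, with lasers damaging the first hit actor.
; SetDeviation adds random spread on yaw or roll, depending on the controller's top-camera state.
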(event `Start Firing`
  (`self.FireWeapon`)
  (`KismetSystemLibrary.K2_SetTimer` null "FireWeapon" (/ 1.0 (`self.FireRate`)) true))

(event `Stop Firing`
  (`KismetSystemLibrary.K2_ClearTimer` null "FireWeapon"))

(event `self.ReceiveBeginPlay`
  (if (not (`self.Laser`))
    (for _ (range (+ (`self.MagazineSize`) 1))
      (bind _returnvalue (`|SpawnActorFromClass` "/Game/10_Blueprints/13_Weapons/BP_ParentProjectile.BP_ParentProjectile_C" (`KismetMathLibrary.MakeTransform` (0.0 0.0 0.0)) "AlwaysSpawn" "OverrideRootScale" (`self.GetOwner`) 100.0 (`self.BaseDamage`) (`self.CriticalDamage`) null))
      (`KismetArrayLibrary.Array_Add` (`self.Magazine`) _returnvalue))))

(fn `FireWeapon`
  (locals (Transform_Local :type "Transform Structure"))
  (bind _magazine (`self.Magazine`))
  (bind _barrelsarray (`self.BarrelsArray`))
  (bind _magazineindex (`self.MagazineIndex`))
  (bind _magazineindex_2 (`self.MagazineIndex`))
  (bind (_output_transform_location _output_transform_rotation) (`KismetMathLibrary.BreakTransform` (`self.SetDeviation` (`local.Transform_Local`))))
  (bind _output (`|GetArrayItem` _magazine _magazineindex))
  (switch `/Game/10_Blueprints/13_Weapons/FiringMode_Enum` (`self.FiringMode`)
    (:`NewEnumerator2`
      (set `local.Transform_Local` (`SceneComponent.K2_GetComponentToWorld` (`self.MainBarrel`)))
      (if (`self.Laser`) :!label _label
        (bind _outhits (`KismetSystemLibrary.BoxTraceMulti` :`Start` _output_transform_location :`End` (+ _output_transform_location (* (`KismetMathLibrary.GetForwardVector` _output_transform_rotation) (`self.LaserRange`))) :`HalfSize` (`self.LaserSize`) :`TraceChannel` "TraceTypeQuery3" :`DrawDebugType` "ForDuration" :`DrawTime` 1.0))
        (if (> (`KismetArrayLibrary.Array_LastIndex` _outhits) -1)
          (bind (_output_bblockinghit _output_binitialoverlap _output_time _output_distance _output_location _output_impactpoint _output_normal _output_impactnormal _output_physmat _output_hitactor _output_hitcomponent) (`GameplayStatics.BreakHitResult` (`|GetArrayItem` _outhits)))
          (`/Game/20_Data/Lib_RetroGun.TestAndInflictDamages` self _output_hitactor _output_hitcomponent (`self.BaseDamage`) (`self.CriticalDamage`)))
        (else
          (`self.K2_SetActorTransform` _output (`self.SetDeviation` (`local.Transform_Local`)) false true)
          (`/Game/20_Data/Lib_RetroGun.EnableActor` _output true)
          (set `self.MagazineIndex` (`self.SetArrayIndex` (+ _magazineindex 1) (`KismetArrayLibrary.Array_LastIndex` _magazine))))))
    (:`NewEnumerator1`
      (set `local.Transform_Local` (`SceneComponent.K2_GetComponentToWorld` (`|GetArrayItem` _barrelsarray _magazineindex_2)))
      (`|ExecutionSequence`
        (:`then_0`
          (goto _label))
        (:`then_1`
          (set `self.BarrelIndex` (`self.SetArrayIndex` _magazineindex_2 (`KismetArrayLibrary.Array_LastIndex` _barrelsarray))))))
    (:`NewEnumerator0`
      (for _array_element _barrelsarray
        (set `local.Transform_Local` (`SceneComponent.K2_GetComponentToWorld` _array_element))
        (goto _label)))))

(fn `SetArrayIndex`
  (params (CurrentIndex :type Integer) (LastIndex :type Integer))
  (returns (NewIndex :type Integer))
  (bind _returnvalue (+ CurrentIndex 1))
  (if (> _returnvalue LastIndex)
    (return 0)
    (else
      (return _returnvalue))))

(fn `SetDeviation`
  (params (`Input Tranform` :type "Transform Structure"))
  (returns (`Output Transform` :type "Transform Structure"))
  (bind _deviation (`self.Deviation`))
  (bind _returnvalue (`KismetMathLibrary.RandomFloatInRange` (* _deviation -1.0) _deviation))
  (if (`/Game/10_Blueprints/11_PlayerPawn/BP_RetroController.CameraOnTop` (`self.Controller_Ref`))
    (return (`KismetMathLibrary.MakeTransform` `Input Tranform_Location` (`KismetMathLibrary.ComposeRotators` `Input Tranform_Rotation` (`KismetMathLibrary.MakeRotator` 0.0 0.0 _returnvalue)) `Input Tranform_Scale`))
    (else
      (return (`KismetMathLibrary.MakeTransform` `Input Tranform_Location` (`KismetMathLibrary.ComposeRotators` `Input Tranform_Rotation` (`KismetMathLibrary.MakeRotator` _returnvalue)) `Input Tranform_Scale`)))))

(fn `UserConstructionScript`
  (bind _asbp_retro_controller (cast `/Game/10_Blueprints/11_PlayerPawn/BP_RetroController` (`Pawn.GetController` (`Actor.Instigator` (`self.GetOwner`)))))
  (set `self.Controller_Ref` _asbp_retro_controller))
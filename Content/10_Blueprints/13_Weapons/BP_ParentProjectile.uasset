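; Base projectile actor that flies forward and deals base or critical damage to what its mesh overlaps.
; Construction caches the owner instigator's retro controller and the game instance, then starts the actor disabled.
; Each tick it moves with sweep at its speed plus the game instance's camera speed.
; It disables itself, rather than being destroyed, after a successful hit or upon passing the viewport's maximum X or Y edge.
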(event `self.ReceiveTick`
  (params (DeltaSeconds :type "Float (single-precision)"))
  (bind (_returnvalue_x _returnvalue_y) (`KismetMathLibrary.BreakVector2D` (`WidgetLayoutLibrary.GetViewportSize`)))
  (bind _screenposition (`GameplayStatics.ProjectWorldToScreen` (`self.Controller_Ref`) (`self.K2_GetActorLocation`)))
  (if (or (> (`KismetMathLibrary.BreakVector2D` _screenposition) _returnvalue_x) (> (`.Y` (`KismetMathLibrary.BreakVector2D` _screenposition)) _returnvalue_y))
    (`/Game/20_Data/Lib_RetroGun.EnableActor` self)
    (else
      (`self.K2_AddActorWorldOffset` (* (`self.GetActorForwardVector`) (* (+ (`self.Speed`) (`/Game/10_Blueprints/BP_RetroInstance.CameraSpeed` (`self.GameInstance_Ref`))) 100.0 (`GameplayStatics.GetWorldDeltaSeconds`))) true))))

(event `self.StaticMesh.OnComponentBeginOverlap`
  (params (OverlappedComponent :type "PrimitiveComponent Object Reference") (OtherActor :type "Actor Object Reference") (OtherComp :type "PrimitiveComponent Object Reference") (OtherBodyIndex :type Integer) (bFromSweep :type Boolean) (SweepResult :type "HitResult Structure (by ref)"))
  (bind _positive (`/Game/20_Data/Lib_RetroGun.TestAndInflictDamages` self OtherActor OtherComp (`self.BaseDamage`) (`self.CriticalDamage`)))
  (if _positive
    (`/Game/20_Data/Lib_RetroGun.EnableActor` self)))

(fn `UserConstructionScript`
  (bind _asbp_retro_controller (cast `/Game/10_Blueprints/11_PlayerPawn/BP_RetroController` (`Pawn.GetController` (`Actor.Instigator` (`self.GetOwner`)))))
  (set `self.Controller_Ref` _asbp_retro_controller)
  (bind _asbp_retro_instance (cast `/Game/10_Blueprints/BP_RetroInstance` (`GameplayStatics.GetGameInstance`)))
  (set `self.GameInstance_Ref` _asbp_retro_instance)
  (`/Game/20_Data/Lib_RetroGun.EnableActor` self))